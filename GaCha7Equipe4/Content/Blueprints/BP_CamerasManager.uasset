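; BP_CamerasManager switches the view between a construction camera and the player hippo's camera.
; On BeginPlay it caches the construction camera's start transform and the player camera, then runs construction activation followed immediately by player activation.
; Construction activation destroys any death or victory camera actors and resets the construction camera.
; Player activation eases the construction camera to the player camera's transform over one second, then activates the player camera.
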(event `self.ReceiveBeginPlay`
  (bind _construction_camera (`self.Construction Camera`))
  (bind _asbp_player_hippo (cast `/Game/Blueprints/Player/BP_Player_Hippo` (`GameplayStatics.GetPlayerPawn` 0)))
  (bind _output_get (set `self.Player Camera` (`/Game/Blueprints/Player/BP_Player_Hippo.Camera` _asbp_player_hippo)))
  (`ActorComponent.Deactivate` _output_get)
  (`ActorComponent.Deactivate` (`CameraActor.CameraComponent` _construction_camera))
  (set `self.C Camera Start Location` (`self.K2_GetActorLocation` _construction_camera))
  (set `self.C Camera Start Rotator` (`self.K2_GetActorRotation` _construction_camera))
  (`self.Activate Construction Camera`)
  (`self.Activate Player Camera`))

(event `Activate Construction Camera`
  (`|ExecutionSequence`
    (:`then_0`
      (`/Engine/EditorBlueprintResources/StandardMacros.IsValid` (`self.Death Camera`)
        (:`Is Valid`
          (`self.K2_DestroyActor` (`ActorComponent.GetOwner` (`self.Death Camera`))))))
    (:`then_1`
      (`/Engine/EditorBlueprintResources/StandardMacros.IsValid` (`self.VictoryCamera`)
        (:`Is Valid`
          (`self.K2_DestroyActor` (`ActorComponent.GetOwner` (`self.VictoryCamera`))))))
    (:`then_2`
      (`SceneComponent.K2_SetWorldTransform` (`CameraActor.CameraComponent` (`self.Construction Camera`)) (`KismetMathLibrary.MakeTransform` (`self.C Camera Start Location`) (`self.C Camera Start Rotator`)) false false)
      (`ActorComponent.Activate` (`CameraActor.CameraComponent` (`self.Construction Camera`)) false))))

(event `Activate Player Camera`
  (bind _player_camera (`self.Player Camera`))
  (`KismetSystemLibrary.MoveComponentTo` (`CameraActor.CameraComponent` (`self.Construction Camera`)) (`SceneComponent.K2_GetComponentLocation` _player_camera) (`SceneComponent.K2_GetComponentRotation` _player_camera) true true 1.0)
  (`ActorComponent.Activate` (`self.Player Camera`) false)
  (`ActorComponent.SetComponentTickEnabled` (`CameraActor.CameraComponent` (`self.Construction Camera`)) false))

(fn `UserConstructionScript`)