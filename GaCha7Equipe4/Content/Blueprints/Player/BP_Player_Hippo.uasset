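; BP_Player_Hippo is the hippo player Blueprint, a physics ball rolled by camera-relative impulses, with horizontal speed capped.
; Mouse input rotates the spring arm, clamping pitch and adjusting arm length with it.
; A downward line trace on Tick sets OnGround, which gates a jump whose impulse scales with current speed.
; A dash impulse exists but is not connected to any event.
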(event `InputAxis|Look Up / Down Mouse`
  (params (AxisValue :type "Float (single-precision)"))
  (bind _springarm (`self.SpringArm`))
  (bind (_relativerotation_roll _relativerotation_pitch _relativerotation_yaw) (`KismetMathLibrary.BreakRotator` (`SceneComponent.RelativeRotation` _springarm)))
  (bind _returnvalue (`KismetMathLibrary.FClamp` (+ _relativerotation_pitch (* AxisValue -1.0)) -50.0 -10.0))
  ;[1 0.2904 0.2705] Contrôle Caméra
  (`SceneComponent.K2_SetRelativeRotation` _springarm (`KismetMathLibrary.MakeRotator` _relativerotation_roll _returnvalue _relativerotation_yaw) false false)
  (set `SpringArmComponent.TargetArmLength` (+ (`self.fFirstCameraArmLength`) (* (- (/ _returnvalue -45.0) 1.0) 100.0)) (`self.SpringArm`)))

(event `InputAxis|Turn Right / Left Mouse`
  (params (AxisValue :type "Float (single-precision)"))
  (bind _springarm (`self.SpringArm`))
  (bind (_relativerotation_roll _relativerotation_pitch _relativerotation_yaw) (`KismetMathLibrary.BreakRotator` (`SceneComponent.RelativeRotation` _springarm)))
  ;[1 0.2904 0.2705] Contrôle Caméra
  (`SceneComponent.K2_SetRelativeRotation` _springarm (`KismetMathLibrary.MakeRotator` _relativerotation_roll _relativerotation_pitch (+ AxisValue _relativerotation_yaw)) false false))

(event `self.ReceiveBeginPlay`
  ;[0.2023 1 0.4581] Sauvegarde de la longueur du bras de la caméra
  (set `self.fFirstCameraArmLength` (`SpringArmComponent.TargetArmLength` (`self.SpringArm`))))

(event `self.ReceiveTick`
  (params (DeltaSeconds :type "Float (single-precision)"))
  (bind _returnvalue (`SceneComponent.K2_GetComponentLocation` (`self.PlayerSphere`)))
  ;[0.5122 0.4542 1] Ground Check
  (bind (_outhit _returnvalue_2) (`KismetSystemLibrary.LineTraceSingle` _returnvalue (- _returnvalue (0.0 0.0 60.0)) "TraceTypeQuery1"))
  (set `self.bOnGround` _returnvalue_2))

(event `InputAxis|Move Right / Left`
  (params (AxisValue :type "Float (single-precision)"))
  (bind _playersphere (`self.PlayerSphere`))
  (bind (_returnvalue_roll _returnvalue_pitch _returnvalue_yaw) (`KismetMathLibrary.BreakRotator` (`SpringArmComponent.GetTargetRotation` (`self.SpringArm`))))
  ;[0.3735 1 0.2551] Impulsion Balle
  (`PrimitiveComponent.AddImpulse` (`self.PlayerSphere`) (`KismetMathLibrary.GreaterGreater_VectorRotator` (* (`KismetMathLibrary.MakeVector` (stale `InputAxis|Move Forward / Backward` AxisValue) AxisValue) (`self.fAcceleration`)) (`KismetMathLibrary.MakeRotator` 0.0 0.0 _returnvalue_yaw)) "None" false :!label _label)
  (bind _returnvalue (`PrimitiveComponent.GetPhysicsLinearVelocity` _playersphere "None"))
  (if (> (`KismetMathLibrary.VSize` (`KismetMathLibrary.MakeVector` (.x _returnvalue) (.y _returnvalue))) (`self.fVitesseMax`))
    (bind (_returnvalue_x _returnvalue_y) (`KismetMathLibrary.BreakVector` (* (`KismetMathLibrary.Normal` (`KismetMathLibrary.MakeVector` (.x _returnvalue) (.y _returnvalue))) (`self.fVitesseMax`))))
    (`PrimitiveComponent.SetPhysicsLinearVelocity` _playersphere (`KismetMathLibrary.MakeVector` _returnvalue_x _returnvalue_y (.z _returnvalue)) false "None")))

(event `InputAxis|Move Forward / Backward`
  (params (AxisValue :type "Float (single-precision)"))
  ;[0.3735 1 0.2551] Impulsion Balle
  (goto _label))

(event `InputAction|Jump`
  (params (Key :type "Key Structure"))
  (bind _fjumppower (`self.fJumpPower`))
  ;[0.25 1 1] Saut
  (:`Pressed`
    (bind _returnvalue (`PrimitiveComponent.GetPhysicsLinearVelocity` (`self.PlayerSphere`) "None"))
    (if (`self.bOnGround`)
      (`PrimitiveComponent.AddImpulse` (`self.PlayerSphere`) (`KismetMathLibrary.MakeVector` 0.0 0.0 (`KismetMathLibrary.FClamp` (* (/ (+ (`KismetMathLibrary.VSize` _returnvalue) _fjumppower) (+ (`self.fVitesseMax`) _fjumppower)) _fjumppower) 0.0 (`self.fJumpPower`))) "None" true))))

(event `InputAction|Dash`
  (params (Key :type "Key Structure"))
  ;[0.9114 0.2299 1] Dash
)

(fn `UserConstructionScript`)