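; BP_GameManager runs the tile-based level game, switching between building a level from tile cards and playing it as the hippo.
; It initializes once TileBoard has a current tile, registering with the game instance, spawning BP_EditorManager and creating the menu HUD.
; Tile clicks extend the board and refill the hand, with Play enabled once an end tile exists.
; Mode switches swap music, input, HUD and camera; death and finish show end screens.
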(event `Init`
  (bind _asbp_game_instance (cast `/Game/Blueprints/BP_GameInstance` (`GameplayStatics.GetGameInstance`)))
  (set `/Game/Blueprints/BP_GameInstance.gameManager` self _asbp_game_instance)
  (bind _returnvalue (`|SpawnActorFromClass` "/Game/Blueprints/BP_EditorManager.BP_EditorManager_C" (`KismetMathLibrary.MakeTransform` (0.0 0.0 0.0)) "Undefined" "OverrideRootScale" null null))
  (bind _asbp_player_hippo (cast `/Game/Blueprints/Player/BP_Player_Hippo` (`GameplayStatics.GetPlayerPawn` 0)))
  (set `self.playerCameraTransform` (`SceneComponent.GetRelativeTransform` (`/Game/Blueprints/Player/BP_Player_Hippo.Camera` _asbp_player_hippo)))
  (add `/Game/Blueprints/Player/BP_Player_Hippo.OnPlayerGoBelowHeight` _asbp_player_hippo (delegate `HandlePlayerDeath`))
  (set `self.editorManager` _returnvalue)
  (bind _returnvalue_2 (`|CreateWidget` "/Game/Blueprints/WBP/WBP_Menu.WBP_Menu_C"))
  (set `self.HUD` _returnvalue_2)
  (`UserWidget.AddToViewport` _returnvalue_2 0)
  (`Widget.SetIsEnabled` (`/Game/Blueprints/WBP/WBP_Menu.WBP_PlayButton` _returnvalue_2) false)
  (add `/Game/Blueprints/WBP/WBP_Menu.OnPlayButtonClicked` _returnvalue_2 (delegate `HandlePlayButton`))
  (add `/Game/Blueprints/WBP/WBP_Menu.OnTileButtonClicked` _returnvalue_2 (delegate `HandleOnButtonClicked`))
  (add `/Game/Blueprints/WBP/WBP_Menu.OnTileButtonHover` _returnvalue_2 (delegate `HandleOnButtonHover`))
  (`self.SwitchToEditorMode`))

(event `self.ReceiveBeginPlay`
  (if (`KismetSystemLibrary.IsValid` (`/Game/Blueprints/BP_TileBoard.CurrentTile` (`self.tileBoard`)))
    (`self.Init`)
    (else
      (add `/Game/Blueprints/BP_TileBoard.OnTileBoardBeginPlay` (`self.tileBoard`) (delegate `CustomEvent`)))))

(event `HandleOnButtonHover`
  (params (tileData :type "/Game/S_TileData Structure")))

(event `HandlePlayerDeath`
  (bind _returnvalue (`|CreateWidget` "/Game/UI/DeathScreen.DeathScreen_C"))
  (`UserWidget.AddToViewport` _returnvalue 0)
  (set `PlayerController.bShowMouseCursor` true (`GameplayStatics.GetPlayerController` 0)))

(event `HandlePlayButton`
  (if (`self.isPlayMode`)
    (`self.SwitchToEditorMode`)
    (else
      (`self.SwitchToPlayMode`))))

(event `EndEditLevel`
  (`Widget.SetIsEnabled` (`/Game/Blueprints/WBP/WBP_Menu.WBP_PlayButton` (`self.HUD`)) true))

(event `HandleOnButtonClicked`
  (params (tileData :type "/Game/S_TileData Structure"))
  (`/Game/Blueprints/BP_TileBoard.SelectCard` (`self.tileBoard`) (`.direction_9_A545F7AF4A84555F6CBB05A81A4A74F3` (break `/Game/S_TileData` tileData)))
  (`self.FillHand`)
  (if (`KismetSystemLibrary.IsValid` (`/Game/Blueprints/BP_TileBoard.EndTile` (`self.tileBoard`)))
    (`self.EndEditLevel`)))

(event `CustomEvent`
  (`self.Init`))

(event `SwitchToEditorMode`
  (bind _returnvalue (`GameplayStatics.GetPlayerController` 0))
  (bind _musique (`self.Musique`))
  (`AudioComponent.SetSound` _musique null)
  (`AudioComponent.Play` _musique 0.0)
  (`Widget.SetVisibility` (`self.HUD`) "Visible")
  (set `PlayerController.bShowMouseCursor` true _returnvalue)
  (`WidgetBlueprintLibrary.SetInputMode_UIOnlyEx` _returnvalue null)
  (set `self.isPlayMode` false)
  (`self.StartEditorPhase`))

(event `StartEditorPhase`
  (bind _asbp_player_hippo (cast `/Game/Blueprints/Player/BP_Player_Hippo` (`GameplayStatics.GetPlayerPawn` 0)))
  (`self.K2_SetActorLocation` _asbp_player_hippo (+ (.location (`self.GetTransform` (`/Game/Blueprints/BP_TileBoard.CurrentTile` (`self.tileBoard`)))) (0.0 0.0 100.0)) false false)
  (`self.FillHand`)
  (`/Game/Blueprints/BP_EditorManager.Set Editor Camera Location` (`self.editorManager`)))

(event `SwitchToPlayMode`
  (bind _returnvalue (`GameplayStatics.GetPlayerController` 0))
  (bind (_playercameratransform_location _playercameratransform_rotation) (`KismetMathLibrary.BreakTransform` (`self.playerCameraTransform`)))
  (bind _musique (`self.Musique`))
  (`AudioComponent.SetSound` _musique "/Game/Cue2/PRINT_RUN_Cue.PRINT_RUN_Cue")
  (`AudioComponent.Play` _musique 0.0)
  (set `PlayerController.bShowMouseCursor` false _returnvalue)
  (`WidgetBlueprintLibrary.SetInputMode_GameOnly` _returnvalue)
  (`Widget.SetVisibility` (`self.HUD`) "Hidden")
  (`self.HideEveryEditorHints`)
  (bind _asbp_player_hippo (cast `/Game/Blueprints/Player/BP_Player_Hippo` (`GameplayStatics.GetPlayerPawn` 0)))
  (`KismetSystemLibrary.MoveComponentTo` (`/Game/Blueprints/Player/BP_Player_Hippo.Camera` _asbp_player_hippo) _playercameratransform_location _playercameratransform_rotation true true 1.0)
  (set `self.isPlayMode` true))

(event `HandleNotInitializedYet`
  (`self.StartEditorPhase`))

(event `OnPlayerFinishLevel`
  (bind _returnvalue (`|CreateWidget` "/Game/UI/Play_again.Play_again_C"))
  (`UserWidget.AddToViewport` _returnvalue 0)
  (set `PlayerController.bShowMouseCursor` true (`GameplayStatics.GetPlayerController` 0)))

(event `FillHand`
  (bind _tileboard (`self.tileBoard`))
  (`/Game/Blueprints/BP_TileBoard.GetCards` _tileboard)
  (`/Game/Blueprints/WBP/WBP_Menu.SetTiles` (`self.HUD`) (`/Game/Blueprints/BP_TileBoard.ForwardTileClass` _tileboard) (`/Game/Blueprints/BP_TileBoard.LeftTileClass` _tileboard) (`/Game/Blueprints/BP_TileBoard.RightTileClass` _tileboard)))

(event `HideEveryEditorHints`
  (bind _tileboard (`self.tileBoard`))
  (`SceneComponent.SetVisibility` (`/Game/Blueprints/BP_TileBoard.Board` _tileboard) false false)
  (for _array_element (`/Game/Blueprints/BP_TileBoard.Tiles` _tileboard)
    (`/Game/Blueprints/BP_BaseTile.DisableHints` _array_element)))

(fn `UserConstructionScript`)