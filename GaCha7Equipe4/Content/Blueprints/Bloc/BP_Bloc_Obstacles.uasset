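; Map block actor that fills itself with obstacle actors at game start, based on difficulty and category.
; On BeginPlay it registers each configured obstacle's class, difficulty, size and category, with short delays around that step.
; CreationObstacles then calls PopulateMap and walks the resulting index grid.
; Each non-negative cell spawns its obstacle on a 100-unit grid around the block, offset by obstacle size.
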(event `self.ReceiveBeginPlay`
  (set `self.Categorie` (`self.BP_Categorie`))
  (`KismetSystemLibrary.Delay` 0.2)
  (for _index (range (`KismetArrayLibrary.Array_Length` (`self.Obstacles`)))
    (bind (_output_actor `_output_difficulté` _output_taille _output_categorie) (break `/Game/Blueprints/Structure/BP_ObstacleStruct` (`|GetArrayItem` (`self.Obstacles`) _index)))
    (`self.AddObstacle` (`KismetMathLibrary.Conv_IntToByte` `_output_difficulté`) (`KismetMathLibrary.Conv_IntToByte` _output_taille) (`GameplayStatics.GetObjectClass` _output_actor) _output_categorie))
  (`KismetSystemLibrary.Delay` 0.2)
  (`self.CreationObstacles`))

(event `self.ReceiveTick`
  (params (DeltaSeconds :type "Float (single-precision)")))

(event `CreationObstacles`
  (bind _returnvalue (`self.GetTransform` self))
  (`self.PopulateMap` (`self.Difficulté`))
  (bind _returnvalue_2 (`self.GetTMap` self))
  (for (_array_element _array_index) _returnvalue_2
    (bind _returnvalue_3 (`self.GetLigne` _array_element))
    (for (_array_element_2 _array_index_2) _returnvalue_3
      (if (>= _array_element_2 0)
        (bind _returnvalue_4 (`self.GetSize` (struct)))
        (bind _returnvalue_5 (`self.GetBP` (`|GetArrayItem` (`self.TObstacleStructs`) _array_element_2)))
        (bind _returnvalue_6 (+ (* (/ _returnvalue_4 2) 100) 50.0))
        (bind _returnvalue_7 (`|SpawnActorFromClass` _returnvalue_5 (`KismetMathLibrary.MakeTransform` (`KismetMathLibrary.MakeVector` (+ _returnvalue_6 (+ (.x (.location _returnvalue)) (- (* _array_index 100) 500.0))) (+ _returnvalue_6 (+ (.y (.location _returnvalue)) (- (* _array_index_2 100) 500.0))) (+ (.z (.location _returnvalue)) 50.0))) "AlwaysSpawn" "OverrideRootScale" null null))))))

(fn `UserConstructionScript`)