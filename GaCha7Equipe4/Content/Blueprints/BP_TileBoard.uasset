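; Tile board actor that scales its board mesh to a rows-by-columns grid and grows a path of tiles from a starting forward tile.
; GetCards checks which directions stay in bounds and asks TileGenerator for one playable tile class.
; SelectCard spawns that class beside the current tile, placed by the current tile's direction and yaw rather than the passed Direction.
; Each new tile records its grid position and becomes current.
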(event `self.ReceiveBeginPlay`
  (if (<= 0 (`KismetArrayLibrary.Array_Length` (`self.Tiles`)))
    (bind _returnvalue (`|SpawnActorFromClass` "/Game/Blueprints/BP_Tile_Forward_01.BP_Tile_Forward_01_C" (`KismetMathLibrary.MakeTransform` (* (`self.FirstTileIndex`) 100.0)) "Undefined" "OverrideRootScale" null null))
    (`KismetArrayLibrary.Array_Add` (`self.Tiles`) _returnvalue)
    (bind _output_get (set `self.CurrentTile` _returnvalue))
    (set `/Game/Blueprints/BP_BaseTile.Position` (`self.FirstTileIndex`) _output_get)
    (`self.GetCards`)))

(event `GetCards`
  (bind _currenttile (`self.CurrentTile`))
  (`|ExecutionSequence`
    (:`then_0`
      (bind _can_spawn (`self.CanSpawnForward` _currenttile))
      (bind _output_get (set `self.SpawnForward` _can_spawn)))
    (:`then_1`
      (bind _can_spawn_2 (`self.CanSpawnLeft` _currenttile))
      (bind _output_get_2 (set `self.SpawnLeft` _can_spawn_2)))
    (:`then_2`
      (bind _can_spawn_3 (`self.Can Spawn Right` _currenttile))
      (bind _output_get_3 (set `self.SpawnRight` _can_spawn_3)))
    (:`then_3`
      (bind _tiles (`/Game/Blueprints/BP_TileGenerator.GetPlayableTiles` (`self.Tile Generator`) 1 (make `/Game/S_PlayableDirections` _output_get _output_get_2 _output_get_3)))
      (bind _output_get_4 (set `self.TileClassesGenerated` _tiles)))))

(event `SelectCard`
  (params (Direction :type "/Game/E_PlayableDirections Enum" :default "NewEnumerator0"))
  (bind _output (`|GetArrayItem` (`self.TileClassesGenerated`)))
  (if (!= _output null)
    (`self.SpawnTile` _output Direction)
    (else
      (`KismetSystemLibrary.PrintString` "Empty" true true (struct :`R` 1.0 :`G` 0.052997 :`A` 1.0)))))

(fn `Can Spawn Right`
  (params (Tile :type "/Game/Blueprints/BP_BaseTile Object Reference"))
  (returns (`Can Spawn` :type Boolean))
  (bind (_returnvalue_roll _returnvalue_pitch _returnvalue_yaw) (`KismetMathLibrary.BreakRotator` (`self.K2_GetActorRotation` Tile)))
  (bind _position_x (`KismetMathLibrary.BreakVector` (`/Game/Blueprints/BP_BaseTile.Position` Tile)))
  (bind (_position_x_2 _position_y) (`KismetMathLibrary.BreakVector` (`/Game/Blueprints/BP_BaseTile.Position` Tile)))
  (switch `/Game/E_PlayableDirections` (`/Game/Blueprints/BP_BaseTile.Direction` Tile)
    (:`NewEnumerator0`
      (return (and (< (+ _position_y 1.0) (`self.TileCollumns`)) (<= _returnvalue_yaw 0.0))))
    (:`NewEnumerator1`
      (return (< (+ _position_x 1.0) (`self.TileRows`))))
    (:`NewEnumerator2`
      (return false))))

(fn `CanSpawnForward`
  (params (Tile :type "/Game/Blueprints/BP_BaseTile Object Reference"))
  (returns (`Can Spawn` :type Boolean))
  (bind (_position_x _position_y) (`KismetMathLibrary.BreakVector` (`/Game/Blueprints/BP_BaseTile.Position` Tile)))
  (bind (_position_x_2 _position_y_2) (`KismetMathLibrary.BreakVector` (`/Game/Blueprints/BP_BaseTile.Position` Tile)))
  (bind _position_x_3 (`KismetMathLibrary.BreakVector` (`/Game/Blueprints/BP_BaseTile.Position` Tile)))
  (switch `/Game/E_PlayableDirections` (`/Game/Blueprints/BP_BaseTile.Direction` Tile)
    (:`NewEnumerator0`
      (return (< (+ _position_x_3 1.0) (`self.TileRows`))))
    (:`NewEnumerator1`
      (return (>= (+ _position_y -1.0) 0.0)))
    (:`NewEnumerator2`
      (return (< (+ _position_y_2 1.0) (`self.TileCollumns`))))))

(fn `CanSpawnLeft`
  (params (Tile :type "/Game/Blueprints/BP_BaseTile Object Reference"))
  (returns (`Can Spawn` :type Boolean))
  (bind (_returnvalue_roll _returnvalue_pitch _returnvalue_yaw) (`KismetMathLibrary.BreakRotator` (`self.K2_GetActorRotation` Tile)))
  (bind _position_x (`KismetMathLibrary.BreakVector` (`/Game/Blueprints/BP_BaseTile.Position` Tile)))
  (bind (_position_x_2 _position_y) (`KismetMathLibrary.BreakVector` (`/Game/Blueprints/BP_BaseTile.Position` Tile)))
  (switch `/Game/E_PlayableDirections` (`/Game/Blueprints/BP_BaseTile.Direction` Tile)
    (:`NewEnumerator0`
      (return (and (>= (+ _position_y -1.0) 0.0) (>= _returnvalue_yaw 0.0))))
    (:`NewEnumerator1`
      (return false))
    (:`NewEnumerator2`
      (return (< (+ _position_x 1.0) (`self.TileRows`))))))

(fn `GetPossibleDirections`
  (returns (Forward :type Boolean) (Left :type Boolean) (Right :type Boolean))
  (return (`self.SpawnForward`) (`self.SpawnLeft`) (`self.SpawnRight`)))

(fn `SpawnForwardTile`
  (params (`Tile Class` :type "/Game/Blueprints/BP_BaseTile Class Reference"))
  (bind (_returnvalue_x _returnvalue_y _returnvalue_z) (`KismetMathLibrary.BreakVector` (`self.K2_GetActorLocation` (`self.CurrentTile`))))
  (bind _returnvalue (`|SpawnActorFromClass` `Tile Class` (`KismetMathLibrary.MakeTransform` (`KismetMathLibrary.MakeVector` (+ _returnvalue_x (* (`self.TileSize`) 100.0)) _returnvalue_y _returnvalue_z)) "Undefined" "OverrideRootScale" null null))
  (set `/Game/Blueprints/BP_BaseTile.Position` (+ (`/Game/Blueprints/BP_BaseTile.Position` (`self.CurrentTile`)) (1.0 0.0 0.0)) _returnvalue)
  (bind _output_get (set `self.CurrentTile` _returnvalue))
  (`KismetArrayLibrary.Array_Add` (`self.Tiles`) _output_get))

(fn `SpawnLeftTile`
  (params (`Tile Class` :type "/Game/Blueprints/BP_BaseTile Class Reference"))
  (bind (_returnvalue_x _returnvalue_y _returnvalue_z) (`KismetMathLibrary.BreakVector` (`self.K2_GetActorLocation` (`self.CurrentTile`))))
  (bind _returnvalue (`|SpawnActorFromClass` `Tile Class` (`KismetMathLibrary.MakeTransform` (`KismetMathLibrary.MakeVector` _returnvalue_x (+ _returnvalue_y (* (`self.TileSize`) -100.0)) _returnvalue_z) (struct :`Yaw` -90.0)) "Undefined" "OverrideRootScale" null null))
  (set `/Game/Blueprints/BP_BaseTile.Position` (+ (`/Game/Blueprints/BP_BaseTile.Position` (`self.CurrentTile`)) (0.0 -1.0 0.0)) _returnvalue)
  (bind _output_get (set `self.CurrentTile` _returnvalue))
  (`KismetArrayLibrary.Array_Add` (`self.Tiles`) _output_get))

(fn `SpawnRightTile`
  (params (`Tile Class` :type "/Game/Blueprints/BP_BaseTile Class Reference"))
  (bind (_returnvalue_x _returnvalue_y _returnvalue_z) (`KismetMathLibrary.BreakVector` (`self.K2_GetActorLocation` (`self.CurrentTile`))))
  (bind _returnvalue (`|SpawnActorFromClass` `Tile Class` (`KismetMathLibrary.MakeTransform` (`KismetMathLibrary.MakeVector` _returnvalue_x (+ _returnvalue_y (* (`self.TileSize`) 100.0)) _returnvalue_z) (struct :`Yaw` 90.0)) "Undefined" "OverrideRootScale" null null))
  (set `/Game/Blueprints/BP_BaseTile.Position` (+ (`/Game/Blueprints/BP_BaseTile.Position` (`self.CurrentTile`)) (0.0 1.0 0.0)) _returnvalue)
  (bind _output_get (set `self.CurrentTile` _returnvalue))
  (`KismetArrayLibrary.Array_Add` (`self.Tiles`) _output_get))

(fn `SpawnTile`
  (params (`Tile Class` :type "/Game/Blueprints/BP_BaseTile Class Reference") (Direction :type "/Game/E_PlayableDirections Enum" :default "NewEnumerator0"))
  (bind (_returnvalue_roll _returnvalue_pitch _returnvalue_yaw) (`KismetMathLibrary.BreakRotator` (`self.K2_GetActorRotation` (`self.CurrentTile`))))
  (bind (_returnvalue_roll_2 _returnvalue_pitch_2 _returnvalue_yaw_2) (`KismetMathLibrary.BreakRotator` (`self.K2_GetActorRotation` (`self.CurrentTile`))))
  (bind (_returnvalue_roll_3 _returnvalue_pitch_3 _returnvalue_yaw_3) (`KismetMathLibrary.BreakRotator` (`self.K2_GetActorRotation` (`self.CurrentTile`))))
  (bind (_returnvalue_roll_4 _returnvalue_pitch_4 _returnvalue_yaw_4) (`KismetMathLibrary.BreakRotator` (`self.K2_GetActorRotation` (`self.CurrentTile`))))
  (bind (_returnvalue_roll_5 _returnvalue_pitch_5 _returnvalue_yaw_5) (`KismetMathLibrary.BreakRotator` (`self.K2_GetActorRotation` (`self.CurrentTile`))))
  (bind (_returnvalue_roll_6 _returnvalue_pitch_6 _returnvalue_yaw_6) (`KismetMathLibrary.BreakRotator` (`self.K2_GetActorRotation` (`self.CurrentTile`))))
  (bind (_returnvalue_roll_7 _returnvalue_pitch_7 _returnvalue_yaw_7) (`KismetMathLibrary.BreakRotator` (`self.K2_GetActorRotation` (`self.CurrentTile`))))
  (bind (_returnvalue_roll_8 _returnvalue_pitch_8 _returnvalue_yaw_8) (`KismetMathLibrary.BreakRotator` (`self.K2_GetActorRotation` (`self.CurrentTile`))))
  (bind (_returnvalue_roll_9 _returnvalue_pitch_9 _returnvalue_yaw_9) (`KismetMathLibrary.BreakRotator` (`self.K2_GetActorRotation` (`self.CurrentTile`))))
  (switch `/Game/E_PlayableDirections` (`/Game/Blueprints/BP_BaseTile.Direction` (`self.CurrentTile`))
    (:`NewEnumerator0`
      ;[1 1 1] Forward
      (`|ExecutionSequence`
        (:`then_0`
          (if (== (`KismetMathLibrary.FTrunc` _returnvalue_yaw_4) 0)
            (`self.SpawnForwardTile` `Tile Class`)
            (return)))
        (:`then_1`
          (if (<= (`KismetMathLibrary.FTrunc` _returnvalue_yaw_5) -90)
            (`self.SpawnLeftTile` `Tile Class`)
            (return)))
        (:`then_2`
          (if (>= (`KismetMathLibrary.FTrunc` _returnvalue_yaw_6) 90)
            (`self.SpawnRightTile` `Tile Class`)
            (return)))
        (:`then_3`
          (return))))
    (:`NewEnumerator1`
      ;[1 1 1] Left
      (`|ExecutionSequence`
        (:`then_0`
          (if (== (`KismetMathLibrary.FTrunc` _returnvalue_yaw_7) 0)
            (`self.SpawnLeftTile` `Tile Class`)
            (return)))
        (:`then_1`
          (if (<= (`KismetMathLibrary.FTrunc` _returnvalue_yaw_8) -90)
            (return)))
        (:`then_2`
          (if (>= (`KismetMathLibrary.FTrunc` _returnvalue_yaw_9) 90)
            (`self.SpawnForwardTile` `Tile Class`)
            (return)))
        (:`then_3`
          (return))))
    (:`NewEnumerator2`
      ;[1 1 1] Right
      (`|ExecutionSequence`
        (:`then_0`
          (if (== (`KismetMathLibrary.FTrunc` _returnvalue_yaw_2) 0)
            (`self.SpawnRightTile` `Tile Class`)
            (return)))
        (:`then_1`
          (if (>= (`KismetMathLibrary.FTrunc` _returnvalue_yaw_3) 90)
            (return)))
        (:`then_2`
          (if (<= (`KismetMathLibrary.FTrunc` _returnvalue_yaw) -90)
            (`self.SpawnForwardTile` `Tile Class`)
            (return)))
        (:`then_3`
          (return))))))

(fn `UserConstructionScript`
  (bind _board (`self.Board`))
  (bind (_returnvalue_x _returnvalue_y _returnvalue_z) (`KismetMathLibrary.BreakVector` (`SceneComponent.K2_GetComponentScale` _board)))
  (`SceneComponent.SetWorldScale3D` _board (`KismetMathLibrary.MakeVector` (* (`self.TileSize`) (`self.TileRows`)) (* (`self.TileSize`) (`self.TileCollumns`)) _returnvalue_z)))