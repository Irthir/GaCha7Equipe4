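; BP_EditorManager is an unfinished manager Blueprint, apparently for setting up a level's camera and start, with nothing wired to BeginPlay.
; SetCamera moves the BP_Player_Hippo camera to a fixed overhead position looking straight down, leaving its start/end tile midpoint math unused.
; StartLevel is an empty stub, with disconnected nodes for spawning player and game mode actors.
; The calls to both functions and a player pawn ownership assignment are also disconnected.
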(event `self.ReceiveBeginPlay`)

(fn `Set Camera`
  (params (startTileTransform :type "Transform Structure") (endTileTransform :type "Transform Structure"))
  (bind _asbp_player_hippo (cast `/Game/Blueprints/Player/BP_Player_Hippo` (`GameplayStatics.GetPlayerPawn` 0)))
  (`SceneComponent.K2_SetWorldLocationAndRotation` (`/Game/Blueprints/Player/BP_Player_Hippo.Camera` _asbp_player_hippo) (`KismetMathLibrary.MakeVector` 4000.0 0.0 10000.0) (struct :`Pitch` -90.0) false false))

(fn `StartLevel`)

(fn `UserConstructionScript`)