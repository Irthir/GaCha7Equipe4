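; BP_TileGenerator supplies random tiles for the forward, left-turn and right-turn playable directions.
; GetPlayableTile picks a random entry from the array matching a direction, and GetPlayableTiles calls it for each allowed direction to return up to three tiles.
; A helper converts the direction flags into an enum list.
; BeginPlay, PoolTileFromArray and the construction script are empty.
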(event `self.ReceiveBeginPlay`)

(event `PoolTileFromArray`)

(fn `ConvertPlayableDirectionsToEnumList`
  (params (PlayableDirections :type "/Game/S_PlayableDirections Structure"))
  (returns (directions :type "Array of /Game/E_PlayableDirections Enum"))
  (locals (result :type "Array of /Game/E_PlayableDirections Enum"))
  (bind (_canmoveforward _canmoveleft _canmoveright) (break `/Game/S_PlayableDirections` PlayableDirections))
  (`|ExecutionSequence`
    (:`then_0`
      (if _canmoveforward
        (`KismetArrayLibrary.Array_Add` (`local.result`) (enumliteral `/Game/E_PlayableDirections` "NewEnumerator0"))))
    (:`then_1`
      (if _canmoveleft
        (`KismetArrayLibrary.Array_Add` (`local.result`) (enumliteral `/Game/E_PlayableDirections` "NewEnumerator1"))))
    (:`then_2`
      (if _canmoveright
        (`KismetArrayLibrary.Array_Add` (`local.result`) (enumliteral `/Game/E_PlayableDirections` "NewEnumerator2"))))
    (:`then_3`
      (return (`local.result`)))))

(fn `GetPlayableTile`
  (params (playableDirections :type "/Game/E_PlayableDirections Enum" :default "NewEnumerator0"))
  (returns (playableTile :type "/Game/S_TileData Structure"))
  (locals (returnTile :type "/Game/S_TileData Structure"))
  (switch `/Game/E_PlayableDirections` playableDirections
    (:`NewEnumerator0`
      (set `local.returnTile` (`KismetArrayLibrary.Array_Random` (`self.ForwardTiles`))))
    (:`NewEnumerator1`
      (set `local.returnTile` (`KismetArrayLibrary.Array_Random` (`self.LeftTurnTiles`))))
    (:`NewEnumerator2`
      (set `local.returnTile` (`KismetArrayLibrary.Array_Random` (`self.RightTurnTiles`)))))
  (return (`local.returnTile`)))

(fn `GetPlayableTiles`
  (params (playableDirections :type "/Game/S_PlayableDirections Structure"))
  (returns (forwardTile :type "/Game/S_TileData Structure") (leftTurnTile :type "/Game/S_TileData Structure") (rightTurnTile :type "/Game/S_TileData Structure"))
  (bind (_canmoveforward _canmoveleft _canmoveright) (break `/Game/S_PlayableDirections` playableDirections))
  (`|ExecutionSequence`
    (:`then_0`
      (if _canmoveforward
        (bind _playabletile (`self.GetPlayableTile` "NewEnumerator0"))))
    (:`then_1`
      (if _canmoveleft
        (bind _playabletile_2 (`self.GetPlayableTile` "NewEnumerator1"))))
    (:`then_2`
      (if _canmoveright
        (bind _playabletile_3 (`self.GetPlayableTile` "NewEnumerator2"))))
    (:`then_3`
      (return _playabletile _playabletile_2 _playabletile_3))))

(fn `UserConstructionScript`)