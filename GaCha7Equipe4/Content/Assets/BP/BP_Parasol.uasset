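; BP_Parasol is a parasol bumper that bounces the player hippo when it overlaps from above.
; On overlap, it checks that the player's sphere is at or above its own Sphere's height.
; It then zeroes the player's vertical velocity while keeping horizontal velocity, so the bounce ignores fall speed.
; A velocity-change impulse along the Sphere's up vector, scaled by FPower, launches the player and a sound plays.
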(event `self.ReceiveActorBeginOverlap`
  (params (OtherActor :type "Actor Object Reference"))
  (bind _asbp_player_hippo (cast `/Game/Blueprints/Player/BP_Player_Hippo` OtherActor))
  (bind _playersphere (`/Game/Blueprints/Player/BP_Player_Hippo.PlayerSphere` _asbp_player_hippo))
  (if (>= (`.Z` (`KismetMathLibrary.BreakVector3f` (`SceneComponent.K2_GetComponentLocation` _playersphere))) (`.Z` (`KismetMathLibrary.BreakVector3f` (`SceneComponent.K2_GetComponentLocation` (`self.Sphere`)))))
    (bind _returnvalue (`PrimitiveComponent.GetPhysicsLinearVelocity` _playersphere "None"))
    (bind (_x _y) (`KismetMathLibrary.BreakVector3f` _returnvalue))
    ;[1 1 1] Bumper
    (`PrimitiveComponent.SetPhysicsLinearVelocity` _playersphere (`KismetMathLibrary.MakeVector` _x _y) false "None")
    (`PrimitiveComponent.AddImpulse` (`/Game/Blueprints/Player/BP_Player_Hippo.PlayerSphere` _asbp_player_hippo) (* (`SceneComponent.GetUpVector` (`self.Sphere`)) (`self.fPower`)) "None" true)
    (`AudioComponent.Play` (`self.Audio`) 0.0)))

(fn `UserConstructionScript`)